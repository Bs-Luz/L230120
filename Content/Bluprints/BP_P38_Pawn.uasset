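; BP_P38_Pawn is a player-steerable P-38 aircraft pawn that flies forward automatically.
; Pitch and Roll axis inputs add clamped local rotations scaled by delta time and RotationSpeed.
; A FlipFlop on Tick alternates between spinning FrontRight with forward movement input and spinning FrontLeft alone, both via RotatePropeller, so each runs every other frame.
; An older AddActorLocalOffset movement node remains unconnected.
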(event EventBeginPlay)

(event Collision|EventActorBeginOverlap
  (params (OtherActor :type Actor%20Object%20Reference)))

(event EventTick
  (params (DeltaSeconds :type Float%20%28single-precision%29))
  (Utilities|FlowControl|FlipFlop
    (:A
      ;[0 0 0] Rotate Left
      (CallFunction|RotatePropeller (Variables|Default|GetFrontRight))
      (Pawn|Input|AddMovementInput (Transformation|GetActorForwardVector) 1.0 false))
    (:B
      ;[0 0 0] Rotate Right
      (CallFunction|RotatePropeller (Variables|Default|GetFrontLeft)))))

(event Input|ActionEvents|InputActionFire
  (params (Key :type Key%20Structure :default "None")))

(event Input|AxisEvents|InputAxisPitch
  (params (AxisValue :type Float%20%28single-precision%29))
  ;[0 0 0] Pitch 회전
  (Transformation|AddActorLocalRotation (Math|Rotator|MakeRotator 0.0 (Math|Float|Clamp(Float) (* AxisValue (Utilities|Time|GetWorldDeltaSeconds) (Variables|속력|GetRotationSpeed)) -1.0) 0.0) false false))

(event Input|AxisEvents|InputAxisRoll
  (params (AxisValue :type Float%20%28single-precision%29))
  ;[0 0 0] Roll 회전
  (Transformation|AddActorLocalRotation (Math|Rotator|MakeRotator (Math|Float|Clamp(Float) (* AxisValue (Utilities|Time|GetWorldDeltaSeconds) (Variables|속력|GetRotationSpeed)) -1.0) 0.0 0.0) false false))

(fn ConstructionScript)

(fn RotatePropeller
  (params (Where :type Scene%20Component%20Object%20Reference))
  (Transformation|AddLocalRotation Where (Math|Rotator|MakeRotator (* (Utilities|Time|GetWorldDeltaSeconds) (Variables|속력|GetPropellaRotationSpeed)) 0.0 0.0) false false))