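; BP_P38 is a P-38 plane actor that spins two front propellers and flies along world X.
; Tick drives a FlipFlop: one frame rolls the right propeller and offsets the actor by MoveSpeed, the next rolls the left propeller.
; A shared RotatePropeller function applies the delta-time-scaled RotationSpeed roll.
; Because the branches alternate, each propeller and the movement update only every other frame, at half the set rates.
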(event EventBeginPlay)

(event Collision|EventActorBeginOverlap
  (params (OtherActor :type Actor%20Object%20Reference)))

(event EventTick
  (params (DeltaSeconds :type Float%20%28single-precision%29))
  (Utilities|FlowControl|FlipFlop
    (:A
      ;[0 0 0] Rotate Left
      (CallFunction|RotatePropeller (Variables|Default|GetFrontRight))
      ;[0 0 0] 이동
      (Transformation|AddActorWorldOffset self (Math|Vector|MakeVector (* (Utilities|Time|GetWorldDeltaSeconds) (Variables|속력|GetMoveSpeed)) 0.0 0.0)))
    (:B
      ;[0 0 0] Rotate Right
      (CallFunction|RotatePropeller (Variables|Default|GetFrontLeft)))))

(fn ConstructionScript)

(fn RotatePropeller
  (params (Where :type Scene%20Component%20Object%20Reference))
  (Transformation|AddLocalRotation Where (Math|Rotator|MakeRotator (* (Utilities|Time|GetWorldDeltaSeconds) (Variables|속력|GetRotationSpeed)) 0.0 0.0) false false))